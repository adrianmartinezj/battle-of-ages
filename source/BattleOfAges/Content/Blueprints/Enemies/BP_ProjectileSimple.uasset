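; BP_ProjectileSimple is the projectile of BP_RangedEnemyCharacter, killing the player on contact.
; Its static mesh overlap calls KillPlayer on a PlayerCharacter, then hands the projectile back to its attach-parent enemy through ResetProjectile rather than destroying it.
; Other overlaps also trigger the reset, except actors whose class is exactly BP_RangedEnemyCharacter or BP_ProjectileSimple, which are ignored.
; The file contains no movement logic.
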(event `self.StaticMesh.OnComponentBeginOverlap`
  (params (OverlappedComponent :type "PrimitiveComponent Object Reference") (OtherActor :type "Actor Object Reference") (OtherComp :type "PrimitiveComponent Object Reference") (OtherBodyIndex :type Integer) (bFromSweep :type Boolean) (SweepResult :type "HitResult Structure (by ref)"))
  (bind _asplayer_character (cast `/Game/Blueprints/Player/PlayerCharacter` OtherActor)
    (:`then`
      (`/Game/Blueprints/Player/PlayerCharacter.KillPlayer` _asplayer_character false)
      (bind _asbp_ranged_enemy_character (cast `/Game/Blueprints/Enemies/BP_RangedEnemyCharacter` (`self.GetAttachParentActor`) :!label _label))
      (`RangedEnemyCharacter.ResetProjectile` _asbp_ranged_enemy_character self))
    (:`CastFailed`
      (if (and (!= (`GameplayStatics.GetObjectClass` OtherActor) "/Game/Blueprints/Enemies/BP_RangedEnemyCharacter.BP_RangedEnemyCharacter_C") (!= (`GameplayStatics.GetObjectClass` OtherActor) "BP_ProjectileSimple_C"))
        (goto _label)))))

(fn `UserConstructionScript`)