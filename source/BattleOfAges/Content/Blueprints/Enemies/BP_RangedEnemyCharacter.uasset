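; Ranged enemy character that kills the player on contact and can be killed through a weak spot.
; HurtCollision overlap calls KillPlayer, while WeakSpotCollision overlap halves the player's velocity, launches them upward and destroys the enemy.
; On destruction it also destroys every projectile in ProjectileList; no firing logic appears in these graphs.
; Contact logic is copied rather than inherited from BaseEnemyCharacter, for simplicity.
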(event `self.HurtCollision.OnComponentBeginOverlap`
  (params (OverlappedComponent :type "PrimitiveComponent Object Reference") (OtherActor :type "Actor Object Reference") (OtherComp :type "PrimitiveComponent Object Reference") (OtherBodyIndex :type Integer) (bFromSweep :type Boolean) (SweepResult :type "HitResult Structure (by ref)"))
  ;[1 0.7787 0.571] Contact Logic, ideally this would be inherited from the BaseEnemyCharacter class (which would also be in C++) but for simplicity I copied / pasted
  (bind _asplayer_character (cast `/Game/Blueprints/Player/PlayerCharacter` OtherActor))
  (`/Game/Blueprints/Player/PlayerCharacter.KillPlayer` _asplayer_character false))

(event `self.WeakSpotCollision.OnComponentBeginOverlap`
  (params (OverlappedComponent :type "PrimitiveComponent Object Reference") (OtherActor :type "Actor Object Reference") (OtherComp :type "PrimitiveComponent Object Reference") (OtherBodyIndex :type Integer) (bFromSweep :type Boolean) (SweepResult :type "HitResult Structure (by ref)"))
  ;[1 0.7787 0.571] Contact Logic, ideally this would be inherited from the BaseEnemyCharacter class (which would also be in C++) but for simplicity I copied / pasted
  (bind _asplayer_character (cast `/Game/Blueprints/Player/PlayerCharacter` OtherActor))
  (bind _charactermovement (`Character.CharacterMovement` _asplayer_character))
  (set `MovementComponent.Velocity` (/ (`MovementComponent.Velocity` _charactermovement) 2.0) _charactermovement)
  (`CharacterMovementComponent.AddImpulse` _charactermovement (0.0 0.0 1000.0) true)
  (`self.KillSelf`))

(event `KillSelf`
  ;[1 0.7787 0.571] Contact Logic, ideally this would be inherited from the BaseEnemyCharacter class (which would also be in C++) but for simplicity I copied / pasted
  (`self.K2_DestroyActor`))

(event `self.ReceiveDestroyed`
  ;[1 0.7787 0.571] Contact Logic, ideally this would be inherited from the BaseEnemyCharacter class (which would also be in C++) but for simplicity I copied / pasted
  (for _array_element (`self.ProjectileList`)
    (`self.K2_DestroyActor` _array_element)))

(fn `UserConstructionScript`)